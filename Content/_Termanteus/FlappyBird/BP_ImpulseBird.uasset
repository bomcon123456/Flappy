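; BP_ImpulseBird is a Flappy Bird actor that propels itself with physics impulses until it hits something.
; While SelfFlight is true, each Tick adds a mass-independent velocity impulse along world -X to the static mesh, without delta-time scaling.
; A Sphere hit on anything other than another BP_ImpulseBird clears SelfFlight and destroys the FlappyComponent, provided that component is still valid.
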(event OnComponentHit(Sphere)
  (params (HitComponent :type Primitive%20Component%20Object%20Reference) (OtherActor :type Actor%20Object%20Reference) (OtherComp :type Primitive%20Component%20Object%20Reference) (NormalImpulse :type Vector :default "0, 0, 0") (Hit :type Hit%20Result%20Structure%20%28by%20ref%29))
  (Utilities|IsValid (Variables|Default|GetFlappyComponent)
    (:Is%20Valid
      (Utilities|Casting|CastToBP_ImpulseBird OtherActor
        (:CastFailed
          (Variables|Default|SetbSelfFlight false)
          (Components|DestroyComponent (Variables|Default|GetFlappyComponent)))))))

(event EventTick
  (params (DeltaSeconds :type Float%20%28single-precision%29))
  (if (Variables|Default|GetbSelfFlight)
    (Physics|AddImpulse (Variables|Default|GetStaticMesh) "-1.000000, 0, 0" "None" true)))

(fn ConstructionScript)