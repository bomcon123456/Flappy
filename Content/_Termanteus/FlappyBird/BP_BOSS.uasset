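; BP_BOSS is a boss actor in a Flappy Bird game that periodically launches BP_ProjectileBird actors.
; On BeginPlay it spawns one bird after a delay, then after another delay starts a looping SpawnBird timer whose interval is randomized once.
; SpawnBird creates scaled-down birds at a random offset from BossMesh's relative location, ignoring collisions.
; Any projectile bird that hits BossMesh is destroyed.
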(event OnComponentHit(BossMesh)
  (params (HitComponent :type Primitive%20Component%20Object%20Reference) (OtherActor :type Actor%20Object%20Reference) (OtherComp :type Primitive%20Component%20Object%20Reference) (NormalImpulse :type Vector :default "0, 0, 0") (Hit :type Hit%20Result%20Structure%20%28by%20ref%29))
  (bind _asbp_projectile_bird (Utilities|Casting|CastToBP_ProjectileBird OtherActor))
  (Actor|DestroyActor _asbp_projectile_bird))

(event EventBeginPlay
  (Utilities|FlowControl|Delay 5.0)
  (CallFunction|SpawnBird)
  (Utilities|FlowControl|Delay 5.0)
  (Utilities|Time|SetTimerbyFunctionName 0 "SpawnBird" (Math|Random|RandomFloatinRange 3.0 6.0) true))

(fn ConstructionScript)

(fn SpawnBird
  (Game|SpawnActorfromClass "/Game/_Termanteus/FlappyBird/BP_ProjectileBird.BP_ProjectileBird_C" (Math|Transform|MakeTransform (- (Variables|/Script/Engine.SceneComponent|GetRelativeLocation (Variables|Default|GetBossMesh)) (Math|Vector|MakeVector (Math|Random|RandomFloatinRange 5e+01 8e+01) (Math|Random|RandomFloatinRange -5e+01 5e+01) (Math|Random|RandomFloatinRange 3e+01 7e+01))) "0, 0,0.000000" "0.300000,0.300000,0.300000") "AlwaysSpawn" self 0))